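; BP_FallingPlat is a platform that falls shortly after the player touches it, then respawns at its starting location.
; A hit from BP_ThirdPersonCharacter turns the cube blue, then after delays it simulates physics, hides, and resets physics, material, transform and visibility.
; The IsRespawning flag blocks retriggering, but is set before the character cast, so a hit from any other actor leaves it latched.
; Falling and ReAppear are empty stubs.
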(event `self.ReceiveBeginPlay`
  ;[1 1 1] GetStartingLocation
  (set `self.location` (`SceneComponent.K2_GetComponentLocation` (`self.Cube`))))

(event `self.Cube.OnComponentHit`
  (params (HitComponent :type "PrimitiveComponent Object Reference") (OtherActor :type "Actor Object Reference") (OtherComp :type "PrimitiveComponent Object Reference") (NormalImpulse :type "Vector Structure") (Hit :type "HitResult Structure (by ref)"))
  ;[1 1 1] TouchingThePlayer
  (if (not (`self.isRespawning`))
    (set `self.isRespawning` true)
    (cast `/Game/ThirdPerson/Blueprints/BP_ThirdPersonCharacter` OtherActor)
    (`PrimitiveComponent.SetMaterial` (`self.Cube`) 0 "/Game/LevelPrototyping/Materials/MI_Solid_Blue.MI_Solid_Blue")
    (`KismetSystemLibrary.Delay` 3.0)
    (`self.Drop`)))

(event `Drop`
  ;[1 1 1] Falling
  (`PrimitiveComponent.SetSimulatePhysics` (`self.Cube`) true)
  (`KismetSystemLibrary.Delay` 2.0)
  (`SceneComponent.SetHiddenInGame` (`self.Cube`) true false)
  (`KismetSystemLibrary.Delay` 2.0)
  (`self.Respawning`))

(event `Respawning`
  ;[1 1 1] Respawning
  (`PrimitiveComponent.SetSimulatePhysics` (`self.Cube`) false)
  (`PrimitiveComponent.SetMaterial` (`self.Cube`) 0 "/Game/LevelPrototyping/Materials/M_Solid.M_Solid")
  (`SceneComponent.K2_SetWorldLocationAndRotation` :`self` (`self.Cube`) :`NewLocation` (`self.location`))
  (`SceneComponent.SetHiddenInGame` (`self.Cube`) false false)
  (set `self.isRespawning` false))

(event `Falling`)

(fn `ReAppear`)

(fn `UserConstructionScript`)