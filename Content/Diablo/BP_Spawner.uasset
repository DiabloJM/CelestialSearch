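; Spawner actor that releases a fixed wave of CubeEnemy actors and spawns a StarPrimitive once all of them are killed.
; A looping timer starts on BeginPlay and, while Activated is set, spawns an enemy at a random SpawnLocations actor until the EnemiesToSpawn cap is reached.
; EnemyKill counts deaths, and when the count matches the cap it prints a message and spawns the star at StarSpawnLocation.
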(event `self.ReceiveBeginPlay`
  ;[1 0.8343 0] Enemy spawn every X seconds
  (`KismetSystemLibrary.K2_SetTimerDelegate` (delegate `Spawn Enemy`) 3.0 true))

(event `Spawn Enemy`
  ;[1 0.8343 0] Enemy spawn every X seconds
  (if (`self.Activated`)
    (if (< (`self.EnemiesSpawned`) (`self.EnemiesToSpawn`))
      (bind _result (`/Engine/EditorBlueprintResources/StandardMacros.IncrementInt` (`self.EnemiesSpawned`))
        (:`  `
          (set `self.EnemiesSpawned` _result)
          (`|SpawnActorFromClass` "/Game/Diablo/CubeEnemy.CubeEnemy_C" (`self.GetTransform` (`KismetArrayLibrary.Array_Random` (`self.SpawnLocations`))) "Undefined" "OverrideRootScale" null null))))))

(event `EnemyKill`
  (bind _enemieskilled (`self.EnemiesKilled`))
  ;[0.03653 0.6813 1] When all enemies are defeated
  (bind _result (`/Engine/EditorBlueprintResources/StandardMacros.IncrementInt` _enemieskilled)
    (:`  `
      (set `self.EnemiesKilled` _result)
      (if (== _enemieskilled (`self.EnemiesToSpawn`))
        (`KismetSystemLibrary.PrintString` "Enemies Killed")
        (`|SpawnActorFromClass` "/Game/Diablo/StarPrimitive.StarPrimitive_C" (`self.GetTransform` (`self.StarSpawnLocation`)) "Undefined" "OverrideRootScale" null null)))))

(fn `UserConstructionScript`)